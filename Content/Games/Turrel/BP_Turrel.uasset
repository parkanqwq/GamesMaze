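; Turret enemy that sweeps for the player, then tracks and shoots them, switching between Patrol and Shot states on Tick.
; Patrol uses a self-restarting timeline to swing the mesh yaw back and forth until a forward sphere trace detects the player character.
; Shot interpolates yaw toward the player while a looping timer fires line traces with explosion effects, applying damage on hits.
; Losing sight clears the timer and resumes patrol from the current rotation.
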(event `StartShoot`
  (bind _returnvalue (`KismetSystemLibrary.K2_SetTimerDelegate` (delegate `CallShootFunc`) 1.0 true))
  (set `self.ShootTimer` _returnvalue))

(event `CallShootFunc`
  (bind _isshoot (`self.Shoot`))
  (if _isshoot
    (bind _asbp_third_person_character (cast `/Game/ThirdPerson/Blueprints/BP_ThirdPersonCharacter` (`GameplayStatics.GetPlayerCharacter` 0)))
    (`GameplayStatics.ApplyDamage` _asbp_third_person_character 10.0)))

(event `self.ReceiveTick`
  (params (DeltaSeconds :type "Float (single-precision)"))
  (bind _skeletalmesh (`self.SkeletalMesh`))
  (bind (_returnvalue_roll _returnvalue_pitch _returnvalue_yaw) (`KismetMathLibrary.BreakRotator` (`SceneComponent.K2_GetComponentRotation` _skeletalmesh)))
  (bind (_returnvalue_roll_2 _returnvalue_pitch_2 _returnvalue_yaw_2) (`KismetMathLibrary.BreakRotator` (`KismetMathLibrary.FindLookAtRotation` (`SceneComponent.K2_GetComponentLocation` (`self.SkeletalMesh`)) (`self.K2_GetActorLocation` (`GameplayStatics.GetPlayerCharacter` 0)))))
  (switch `/Game/Games/Turrel/E_TurretState` (`self.CurrentState`)
    (:`NewEnumerator0`
      (bind _isplayerfind (`self.PlayerSearch`))
      (if _isplayerfind
        (`self.StopPatrol`)
        (set `self.CurrentState` "NewEnumerator1")))
    (:`NewEnumerator1`
      (`SceneComponent.K2_SetWorldRotation` _skeletalmesh (`KismetMathLibrary.RInterpTo` (`KismetMathLibrary.MakeRotator` _returnvalue_roll _returnvalue_pitch _returnvalue_yaw) (`KismetMathLibrary.MakeRotator` _returnvalue_roll _returnvalue_pitch (- _returnvalue_yaw_2 90.0)) (`GameplayStatics.GetWorldDeltaSeconds`)) false false)
      (`|ExecutionSequence`
        (:`then_0`
          (if (not (`self.IsStartShoot`))
            (`self.StartShoot`)
            (set `self.IsStartShoot` true)))
        (:`then_1`
          (bind _isplayerfind_2 (`self.PlayerSearch`))
          (if (not _isplayerfind_2)
            (`KismetSystemLibrary.K2_ClearAndInvalidateTimerHandle` (`self.ShootTimer`))
            (set `self.IsStartShoot` false)
            (set `self.CurrentState` "NewEnumerator0")
            (set `self.TargetRotation` (`self.EndRotation`))
            (set `self.CurrentRotation` (`SceneComponent.K2_GetComponentRotation` (`self.SkeletalMesh`)))
            (set `self.DirectionMove` "Forward")
            (`self.StartPatrol`)))))))

(event `self.ReceiveBeginPlay`
  (bind _output_get (set `self.StartRotation` (`SceneComponent.K2_GetComponentRotation` (`self.SkeletalMesh`))))
  (set `self.EndRotation` (`KismetMathLibrary.MakeRotator` (.roll _output_get) (.pitch _output_get) (+ (.yaw _output_get) 120.0)))
  (set `self.CurrentRotation` (`self.StartRotation`))
  (set `self.TargetRotation` (`self.EndRotation`))
  (`self.StartPatrol`))

(event `StartPatrol`
  (bind (_direction _rotatetrack) (`Timeline|Шкала времени` :!via `PlayFromStart` :!label _label)
    (:`Update`
      (`SceneComponent.K2_SetWorldRotation` (`self.SkeletalMesh`) (`KismetMathLibrary.RLerp` (`self.CurrentRotation`) (`self.TargetRotation`) _rotatetrack) false false))
    (:`Finished`
      (switch `ETimelineDirection` (`self.DirectionMove`)
        (:`Forward`
          (set `self.DirectionMove` "Backward")
          (set `self.TargetRotation` (`self.StartRotation`))
          (set `self.CurrentRotation` (`self.EndRotation`)))
        (:`Backward`
          (set `self.DirectionMove` "Forward")
          (set `self.TargetRotation` (`self.EndRotation`))
          (set `self.CurrentRotation` (`self.StartRotation`))))
      (`self.StartPatrol`))))

(event `StopPatrol`
  (goto _label :!via `Stop`))

(fn `PlayerSearch`
  (returns (IsPlayerFind :type Boolean))
  (bind _scene (`self.Scene`))
  (bind _returnvalue (`SceneComponent.K2_GetComponentLocation` _scene))
  (bind (_outhit _returnvalue_2) (`KismetSystemLibrary.SphereTraceSingle` _returnvalue (+ _returnvalue (* (`SceneComponent.GetForwardVector` _scene) (`self.SearchDistance`))) 10.0 "TraceTypeQuery2"))
  (if _returnvalue_2
    (cast `/Game/ThirdPerson/Blueprints/BP_ThirdPersonCharacter` (`.HitActor` (`GameplayStatics.BreakHitResult` _outhit))
      (:`then`
        (return true))
      (:`CastFailed`
        (return false)))
    (else
      (return false))))

(fn `Shoot`
  (returns (IsShoot :type Boolean))
  (bind _scene (`self.Scene`))
  (bind _returnvalue (`SceneComponent.K2_GetComponentLocation` _scene))
  (bind (_outhit _returnvalue_2) (`KismetSystemLibrary.LineTraceSingle` _returnvalue (+ _returnvalue (* (`SceneComponent.GetForwardVector` _scene) (`self.ShootDistance`))) "TraceTypeQuery2"))
  (`|ExecutionSequence`
    (:`then_0`
      (`GameplayStatics.PlaySoundAtLocation` "/Game/StarterContent/Audio/Explosion01.Explosion01" (`SceneComponent.K2_GetComponentLocation` (`self.Scene`)) (struct) 1.0 1.0 0.0 null null null null)
      (`GameplayStatics.SpawnEmitterAttached` "/Game/StarterContent/Particles/P_Explosion.P_Explosion" (`self.Scene`)))
    (:`then_1`
      (if _returnvalue_2
        (cast `/Game/ThirdPerson/Blueprints/BP_ThirdPersonCharacter` (`.HitActor` (`GameplayStatics.BreakHitResult` _outhit))
          (:`then`
            (return true))
          (:`CastFailed`
            (return false)))
        (else
          (return false))))))

(fn `UserConstructionScript`)
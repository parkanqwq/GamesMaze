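; BP_Lever is an interactable lever that triggers Control on a linked actor, ControledActor.
; Interact calls Control whenever that reference is valid; the first time OnSound is set, it also plays a tractor carburetor sound at the Box and clears the flag.
; Box overlap sets IsCanUse only while OnSound is true and clears it on exit.
; Interact itself does not check IsCanUse.
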(event `/Game/Games/Blueprints/BPI_Interactable.Interact`
  (bind _controledactor (`self.ControledActor`))
  (`/Engine/EditorBlueprintResources/StandardMacros.IsValid` _controledactor
    (:`Is Valid`
      (`/Game/Games/Blueprints/BP_ControlActor.Control` _controledactor)
      (if (`self.OnSound`)
        (`GameplayStatics.PlaySoundAtLocation` "/Game/Games/Music/carburetor_tractor.carburetor_tractor" (`SceneComponent.K2_GetComponentLocation` (`self.Box`)) (struct) 0.6 1.0 0.0 null null null null)
        (set `self.OnSound` false)))))

(event `self.Box.OnComponentBeginOverlap`
  (params (OverlappedComponent :type "PrimitiveComponent Object Reference") (OtherActor :type "Actor Object Reference") (OtherComp :type "PrimitiveComponent Object Reference") (OtherBodyIndex :type Integer) (bFromSweep :type Boolean) (SweepResult :type "HitResult Structure (by ref)"))
  (if (`self.OnSound`)
    (set `self.IsCanUse` true)))

(event `self.Box.OnComponentEndOverlap`
  (params (OverlappedComponent :type "PrimitiveComponent Object Reference") (OtherActor :type "Actor Object Reference") (OtherComp :type "PrimitiveComponent Object Reference") (OtherBodyIndex :type Integer))
  (set `self.IsCanUse` false))

(fn `UserConstructionScript`)
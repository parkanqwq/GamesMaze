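; BP_Door is a door actor that swings open with a timeline animation when interacted with.
; Interact passes through a Gate, which the Control event opens, then plays the timeline from the start.
; The timeline lerps actor rotation from BlockDoor to OpenDoorRotation and, on finish, overwrites BlockDoor with a fixed rotation.
; Nothing in the graph closes the Gate again.
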(event `/Game/Games/Blueprints/BPI_Interactable.Interact`
  (`/Engine/EditorBlueprintResources/StandardMacros.Gate` true :!label _label
    (:`Exit`
      (bind (_direction `_новая_дорожка_0`) (`Timeline|Шкала времени` :!via `PlayFromStart`)
        (:`Update`
          (`self.K2_SetActorRotation` (`KismetMathLibrary.RLerp` (`self.BlockDoor`) (`self.OpenDoorRotation`) `_новая_дорожка_0`)))
        (:`Finished`
          (set `self.BlockDoor` (struct :`Yaw` -90.0)))))))

(event `self.Control`
  (goto _label :!via `Open`))

(fn `UserConstructionScript`
  (`parent.UserConstructionScript`))
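; BP_LiftingGate is a gate actor that alternately raises and lowers itself each time it is triggered.
; Its Control event sets a 1.5-second timer that calls Open/Close, where a FlipFlop picks one of two timelines.
; Each timeline update shifts the actor's Z by a fixed step, up or down, so total travel depends on update count rather than a timeline curve.
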(event `self.Control`
  (`KismetSystemLibrary.K2_SetTimerDelegate` (delegate `Open/Close`) 1.5))

(event `Open/Close`
  (bind (_returnvalue_x _returnvalue_y _returnvalue_z) (`KismetMathLibrary.BreakVector` (`self.K2_GetActorLocation`)))
  (bind (_returnvalue_x_2 _returnvalue_y_2 _returnvalue_z_2) (`KismetMathLibrary.BreakVector` (`self.K2_GetActorLocation`)))
  (`/Engine/EditorBlueprintResources/StandardMacros.FlipFlop`
    (:`A`
      (`Timeline|Шкала времени` :!via `PlayFromStart`
        (:`Update`
          (`self.K2_SetActorLocation` (`KismetMathLibrary.MakeVector` _returnvalue_x_2 _returnvalue_y_2 (+ _returnvalue_z_2 3.0))))))
    (:`B`
      (`Timeline|Шкала времени_0` :!via `PlayFromStart`
        (:`Update`
          (`self.K2_SetActorLocation` (`KismetMathLibrary.MakeVector` _returnvalue_x _returnvalue_y (- _returnvalue_z 3.0))))))))

(fn `UserConstructionScript`
  (`parent.UserConstructionScript`))